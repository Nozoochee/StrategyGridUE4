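; Game mode for a turn-based grid strategy match between a human player and a simple AI, each starting with one unit at either end of the grid.
; It alternates turns through player turn-end dispatchers, runs building effects between turns and binds input and HUD events for the human's turn.
; A turn-phase state machine drives tile selection, using highlighted reachable tiles to move units via AIMoveTo or place new units and buildings.
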(event EventBeginPlay
  (bind _returnvalue (Actor|GetActorOfClass "/Game/Core/Grid/BP/BP_GridManager.BP_GridManager_C"))
  (Variables|Default|SetGrid _returnvalue)
  (bind _asbp_grid_player_controller (Utilities|Casting|CastToBP_GridPlayerController (Game|GetPlayerController 0)))
  (Variables|HumanPlayer|SetGridPlayerController _asbp_grid_player_controller)
  ;[0 0 0] Have to wait for PlayerController to spawn HUD
  (Utilities|FlowControl|Delay 0.2)
  (CallFunction|StartMatch 2))

(fn ConstructionScript)

(fn HandleSelection
  (params (Selection :type BP%20Tile%20Object%20Reference))
  (switch Utilities|FlowControl|Switch|SwitchonE_TurnPhase (Variables|Default|GetCurrentTurnPhase)
    (:NewEnumerator0
      ;[0 0 0] Clicking on a tile with your own unit on it assumes that you want to move that unit to a new place
      (if (== (Variables|/Game/Core/Grid/BP/BP_Tile.BP_Tile_C|GetOwningPlayer Selection) (Variables|Default|GetCurrentPlayer))
        (bind _asbp_base_unit (Utilities|Casting|CastToBP_BaseUnit (Variables|/Game/Core/Grid/BP/BP_Tile.BP_Tile_C|GetActorThatIsStandingOnThisTile Selection)))
        (Variables|HumanPlayer|SetPlayerSelectedUnit _asbp_base_unit)
        (bind _tiles (Default|GetReachableTiles (Variables|Default|GetGrid) (Variables|Default|GetCurrentPlayer) false))
        (bind _output_get (Variables|HumanPlayer|SetPlayerReachableTiles _tiles))
        (for _array_element _output_get
          (Default|SetTmpColor _array_element))
        (CallFunction|ChangeTurnPhase "NewEnumerator3")))
    (:NewEnumerator3
      ;[0 0 0] HumanMoveTarget is the phase where you select the new tile the unit will go to
      (if (Utilities|Array|ContainsItem (Variables|HumanPlayer|GetPlayerReachableTiles) Selection)
        (for _array_element_2 (Variables|HumanPlayer|GetPlayerReachableTiles)
          (Default|ClearTmpColor _array_element_2))
        (CallFunction|MoveUnittoTile (Variables|HumanPlayer|GetPlayerSelectedUnit) Selection)
        (CallFunction|ChangeTurnPhase "NewEnumerator0")))
    (:NewEnumerator4
      ;[0 0 0] HumanPlaceActor is reached when you try and place a new unit/build a building.
      ; Places the unit/building where  you clicked
      (if (Utilities|Array|ContainsItem (Variables|HumanPlayer|GetPlayerReachableTiles) Selection)
        (for _array_element_3 (Variables|HumanPlayer|GetPlayerReachableTiles)
          (Default|ClearTmpColor _array_element_3))
        (CallFunction|SetActoronField Selection (Variables|HumanPlayer|GetClickedActor))
        (CallFunction|ChangeTurnPhase "NewEnumerator0")))))

(fn PlacePlayers
  (bind _values (Utilities|Map|Values (Variables|/Game/Core/Grid/BP/BP_GridManager.BP_GridManager_C|GetTileMap (Variables|Default|GetGrid))))
  (LocalVariables|Setloc_gridIndeces _values)
  (LocalVariables|Setloc_startingTiles (Utilities|Array|MakeArray (Utilities|Array|Get(acopy) (LocalVariables|Getloc_gridIndeces)) (Utilities|Array|Get(acopy) (LocalVariables|Getloc_gridIndeces) (- (Utilities|Array|Length (LocalVariables|Getloc_gridIndeces)) 1))))
  ;[0 0 0] Give each player a unit and place it on their starting tile
  (for (_array_element _array_index) (Variables|Default|GetPlayers)
    (LocalVariables|Setloc_player _array_element)
    (LocalVariables|Setloc_tile (Utilities|Array|Get(acopy) (LocalVariables|Getloc_startingTiles) _array_index))
    (bind _returnvalue (Game|SpawnActorfromClass "/Game/Core/Placeables/Units/BP/BP_BaseUnit.BP_BaseUnit_C" (Math|Transform|MakeTransform "0, 0, 0" "0, 0, 0" "1,1,1") "Undefined" 0 0))
    (bind _output_get (LocalVariables|Setloc_spawnedUnit _returnvalue))
    (Class|BPIPlaceable|SetOwningPlayer(Message) _output_get (LocalVariables|Getloc_player))
    (Default|PlaceUnitonTile (Variables|Default|GetGrid) (LocalVariables|Getloc_spawnedUnit) (LocalVariables|Getloc_tile))
    (Default|AddUnit (LocalVariables|Getloc_player) (LocalVariables|Getloc_spawnedUnit))))

(fn BindPlayerEvents
  (bind _gridplayercontroller (Variables|HumanPlayer|GetGridPlayerController))
  ;[0 0 0] Binds to all the necessary event dispatcher to make a human player do their turn
  (EventDispatchers|BindEventtoOnTileSelection _gridplayercontroller (EventDispatchers|CreateEvent :!event HandleSelection))
  (EventDispatchers|BindEventtoOnEntryClicked (Variables|/Game/Core/Players/Human/BP_GridPlayerController.BP_GridPlayerController_C|GetPlayerHUD _gridplayercontroller) (EventDispatchers|CreateEvent :!event Custom|OnEntryClicked_Event)))

(fn UnbindPlayerEvents
  (bind _gridplayercontroller (Variables|HumanPlayer|GetGridPlayerController))
  ;[0 0 0] Unbinds all the events that were bound in BindPlayerEvents
  (EventDispatchers|UnbindEventfromOnTileSelection _gridplayercontroller (EventDispatchers|CreateEvent :!event HandleSelection))
  (EventDispatchers|UnbindEventfromOnEntryClicked (Variables|/Game/Core/Players/Human/BP_GridPlayerController.BP_GridPlayerController_C|GetPlayerHUD _gridplayercontroller) (EventDispatchers|CreateEvent :!event Custom|OnEntryClicked_Event)))

(fn SetActoronField
  (params (Selection :type BP%20Tile%20Object%20Reference) (ClassToSpawn :type Actor%20Class%20Reference))
  (bind _returnvalue (Game|SpawnActorfromClass ClassToSpawn (Math|Transform|MakeTransform "0, 0, 0" "0, 0, 0" "1,1,1") "Undefined" 0 0))
  (bind _output_get (LocalVariables|SetLoc_ClickedActor _returnvalue))
  (Class|BPIPlaceable|SetOwningPlayer(Message) _output_get (Variables|Default|GetCurrentPlayer))
  (Class|BPIPlaceable|SetTile(Message) (LocalVariables|GetLoc_ClickedActor) Selection)
  (bind _type (Class|BPIPlaceable|GetType(Message) (LocalVariables|GetLoc_ClickedActor)))
  (if (Utilities|Enum|Equal(Enum) _type "NewEnumerator0")
    (bind _returnvalue_2 (Default|PlaceUnitonTile (Variables|Default|GetGrid) (LocalVariables|GetLoc_ClickedActor) Selection))
    (if _returnvalue_2
      (bind _asbp_base_unit (Utilities|Casting|CastToBP_BaseUnit (LocalVariables|GetLoc_ClickedActor)))
      (Default|AddUnit (Variables|Default|GetCurrentPlayer) _asbp_base_unit))
    (else
      (Default|PlaceBuildingonTile (Variables|Default|GetGrid) (LocalVariables|GetLoc_ClickedActor) Selection))))

(event Custom|EndTurn
  ;[0.006593 0 1] Turn End
  (Default|RunBuildingEffects (Variables|Default|GetGrid))
  (if (== (Variables|Default|GetCurrentPlayer) (Game|Player|GetPlayerPawn 0))
    (HumanPlayer|UnbindPlayerEvents))
  (Math|Integer|IncrementInt (Variables|Default|GetCurrentTurn)
    (:%20%20
      (CallFunction|ChangeTurnPhase "NewEnumerator2")
      (bind _output_get (Variables|Default|SetCurrentPlayer (Utilities|Array|Get(acopy) (Variables|Default|GetPlayers) (Math|Integer|%(Integer) (Variables|Default|GetCurrentTurn) (Variables|Default|GetMaxPlayers)))))
      (EventDispatchers|AssignOnTurnEnd _output_get (EventDispatchers|CreateEvent :!event Custom|OnTurnEnd_Event))
      (CallFunction|StartNextTurn))))

(event Custom|StartNextTurn
  ;[1 0.09129 0] Turn Start
  (CallFunction|ChangeTurnPhase "NewEnumerator0")
  (if (== (Variables|Default|GetCurrentPlayer) (Game|Player|GetPlayerPawn 0))
    (HumanPlayer|BindPlayerEvents))
  (Default|PlayTurn (Variables|Default|GetCurrentPlayer)))

(event Custom|ChangeTurnPhase
  (params (NewPhase :type E_TurnPhase%20Enum :default "NewEnumerator0"))
  ;[0.07425 1 0] Turn Phase Change
  (bind _output_get (Variables|Default|SetCurrentTurnPhase NewPhase))
  ;;[0 0 0] Used in UI to update text
  (Default|CallOnTurnPhaseChanged _output_get))

(event Custom|OnEntryClicked_Event
  (params (ClickedActor :type Actor%20Class%20Reference))
  ;[0 0 0] On Entry Clicked. Used to build buildings/place units
  (if (Utilities|Enum|NotEqual(Enum) (Variables|Default|GetCurrentTurnPhase) "NewEnumerator4")
    (CallFunction|ChangeTurnPhase "NewEnumerator4"))
  (Variables|HumanPlayer|SetClickedActor ClickedActor)
  ;;[1 1 1] Change color of selectable tiles
  (bind _tiles (Default|GetReachableTiles (Variables|Default|GetGrid) (Variables|Default|GetCurrentPlayer) true))
  (bind _output_get (Variables|HumanPlayer|SetPlayerReachableTiles _tiles))
  (for _array_element _output_get
    (Default|SetTmpColor _array_element)))

(event Custom|OnTurnEnd_Event
  ;[0 0 0] On Turn End
  (EventDispatchers|UnbindEventfromOnTurnEnd (Variables|Default|GetCurrentPlayer) (delegate Custom|OnTurnEnd_Event))
  (CallFunction|EndTurn))

(event Custom|StartMatch
  (params (NumPlayers :type Integer))
  ;[0 0 0] Start match
  (Variables|Default|SetMaxPlayers NumPlayers)
  (Utilities|Array|Add (Variables|Default|GetPlayers) (.AsBP%20Base%20Player (Utilities|Casting|CastToBP_BasePlayer (Game|Player|GetPlayerPawn 0))))
  (bind _returnvalue (Game|SpawnActorfromClass "/Game/Core/Players/AI/BP_AI_Stupid.BP_AI_Stupid_C" (Math|Transform|MakeTransform "0, 0, 0") "Undefined" 0 0))
  (Utilities|Array|Add (Variables|Default|GetPlayers) _returnvalue)
  (CallFunction|PlacePlayers)
  (bind _output_get (Variables|Default|SetCurrentPlayer (Utilities|Array|Get(acopy) (Variables|Default|GetPlayers))))
  (EventDispatchers|AssignOnTurnEnd _output_get (EventDispatchers|CreateEvent :!event Custom|OnTurnEnd_Event))
  (CallFunction|StartNextTurn))

(event Custom|MoveUnitToTile
  (params (Unit :type BP%20Base%20Unit%20Object%20Reference) (NewTile :type BP%20Tile%20Object%20Reference))
  ;[0 0 0] Moves unit to a new tile. Frees the old tile and captures the new one
  (Default|FreeTile (Variables|/Game/Core/Placeables/Units/BP/BP_BaseUnit.BP_BaseUnit_C|GetCurrentTile Unit))
  (AI|AIMoveTo Unit (Transformation|GetActorLocation NewTile) 0 1e+01 false
    (:then
      (Default|FightTile NewTile Unit))))