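; BP_Tile is a grid tile that tracks its occupant, occupancy state and owning player.
; Filling a tile sets its state from the occupant's type and takes that occupant's owner, recoloring a dynamic material for player or AI.
; Fighting always favors the attacker, removing and destroying any defending unit before claiming the tile.
; Freeing keeps ownership, and a temporary highlight saves and restores the previous color.
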(event Custom|FreeTile
  ;[0 0 0] Frees up the tile without changing it's owner
  (Variables|Default|SetActorThatIsStandingOnThisTile 0)
  (Variables|Default|SetState "NewEnumerator0"))

(event Custom|UpdateTileColor
  ;[0.8482 0 1] Color events
  (bind _output_get (Variables|Default|SetTileOwner (select (== (Variables|Default|GetOwningPlayer) (Game|Player|GetPlayerPawn 0)) "NewEnumerator1" "NewEnumerator2")))
  (Rendering|Material|SetVectorParameterValue (Variables|Default|GetMaterialInstance) "Color" (Utilities|Select :Index _output_get :NewEnumerator0 "(R=0.359375,G=0.359375,B=0.359375,A=1.000000)" :NewEnumerator1 "(R=0.000000,G=0.092295,B=1.000000,A=1.000000)" :NewEnumerator2 "(R=1.000000,G=0.008761,B=0.000000,A=1.000000)") :!class /Script/Engine.MaterialInstanceDynamic))

(event Custom|FillTile
  (params (FilledInActor :type Actor%20Object%20Reference))
  ;[0 0 0] Adds actor to the tile. Can be either a Unit or a Building. Then updates the owner
  (bind _output_get (Variables|Default|SetActorThatIsStandingOnThisTile FilledInActor))
  (bind _type (Class|BPIPlaceable|GetType(Message) _output_get))
  (Variables|Default|SetState (select (Utilities|Enum|Equal(Enum) _type "NewEnumerator1") "NewEnumerator2" "NewEnumerator1"))
  (bind _owningplayer (Class|BPIPlaceable|GetOwningPlayer(Message) (Variables|Default|GetActorThatIsStandingOnThisTile)))
  (CallFunction|UpdateOwner _owningplayer))

(event Custom|UpdateOwner
  (params (NewOwningPlayer :type Pawn%20Object%20Reference))
  ;[0 0 0] Updates the owner and color of the tile
  (Variables|Default|SetOwningPlayer NewOwningPlayer)
  (Variables|Default|SetTileOwner (select (== (Variables|Default|GetOwningPlayer) (Game|Player|GetPlayerPawn 0)) "NewEnumerator1" "NewEnumerator2"))
  (CallFunction|UpdateTileColor))

(event Custom|FightTile
  (params (Fighter :type BP%20Base%20Unit%20Object%20Reference))
  (bind _actorthatisstandingonthistile (Variables|Default|GetActorThatIsStandingOnThisTile))
  ;[0 0 0] Engages battle. Currently whoever attacks automatically wins
  (Variables|/Game/Core/Placeables/Units/BP/BP_BaseUnit.BP_BaseUnit_C|SetCurrentTile Fighter self)
  (Utilities|IsValid (Variables|Default|GetActorThatIsStandingOnThisTile)
    (:Is%20Valid
      (bind _asbp_base_player (Utilities|Casting|CastToBP_BasePlayer (Variables|Default|GetOwningPlayer)))
      (bind _asbp_base_unit (Utilities|Casting|CastToBP_BaseUnit _actorthatisstandingonthistile))
      (Utilities|Array|RemoveItem (Variables|/Game/Core/Players/BP_BasePlayer.BP_BasePlayer_C|GetUnitsOnField _asbp_base_player) _asbp_base_unit)
      (Actor|DestroyActor _actorthatisstandingonthistile))
    (:Is%20Not%20Valid
      _))
  (CallFunction|FillTile Fighter))

(event Custom|SetTmpColor
  ;[0.8482 0 1] Color events
  (bind _returnvalue (Rendering|Material|GetVectorParameterValue (Variables|Default|GetMaterialInstance) "Color" :!class /Script/Engine.MaterialInstanceDynamic))
  (Variables|Default|SetOrgColor _returnvalue)
  (Rendering|Material|SetVectorParameterValue (Variables|Default|GetMaterialInstance) "Color" "(R=1.000000,G=0.820370,B=0.000000,A=1.000000)" :!class /Script/Engine.MaterialInstanceDynamic))

(event Custom|ClearTmpColor
  ;[0.8482 0 1] Color events
  (Rendering|Material|SetVectorParameterValue (Variables|Default|GetMaterialInstance) "Color" (Variables|Default|GetOrgColor) :!class /Script/Engine.MaterialInstanceDynamic)
  (if (== (Variables|Default|GetOrgColor) "(R=1.000000,G=0.823529,B=0.000000,A=1.000000)")
    (Development|PrintString "Hello" true true "(R=1.000000,G=0.823529,B=0.000000,A=1.000000)")))

(event EventBeginPlay
  (bind _returnvalue (Rendering|Material|CreateDynamicMaterialInstance (Variables|Default|GetPlane) 0 0 "None" :!class /Script/Engine.PrimitiveComponent))
  (Variables|Default|SetMaterialInstance _returnvalue)
  (Rendering|Material|SetVectorParameterValue (Variables|Default|GetMaterialInstance) "Color" "(R=0.356863,G=0.356863,B=0.356863,A=1.000000)" :!class /Script/Engine.MaterialInstanceDynamic))

(fn ConstructionScript)