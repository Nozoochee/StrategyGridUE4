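; Grid manager for a turn-based game with player-owned tiles, units and buildings.
; On BeginPlay it spawns BP_Tile actors where a child-actor TileChecker allows and maps them by grid index, with an optional instanced-mesh preview from the construction script.
; It answers neighbor and per-player reachable-tile queries from that map and validates unit and building placement.
; Placed buildings are tracked so RunBuildingEffects can add their score to their owners.
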(event Custom|RunBuildingEffects
  ;[0 0 0] Go through all buildings that are on the field and add their score to the owning player. Called when the turn ends from the gamemode
  (for _array_element (Variables|Default|GetBuildings)
    (bind _asbp_base_player (Utilities|Casting|CastToBP_BasePlayer (Variables|/Game/Core/Placeables/Buildings/BP/BP_BaseBuilding.BP_BaseBuilding_C|GetOwningPlayer _array_element)))
    (Variables|/Game/Core/Players/BP_BasePlayer.BP_BasePlayer_C|SetScore _asbp_base_player (+ (Variables|/Game/Core/Players/BP_BasePlayer.BP_BasePlayer_C|GetScore _asbp_base_player) (Variables|/Game/Core/Placeables/Buildings/BP/BP_BaseBuilding.BP_BaseBuilding_C|GetScore _array_element)))))

(event EventBeginPlay
  (Components|InstancedStaticMesh|ClearInstances (Variables|Default|GetInstancedStaticMesh))
  (bind _asbp_tile_checker (Utilities|Casting|CastToBP_TileChecker (Variables|/Script/Engine.ChildActorComponent|GetChildActor (Variables|Default|GetChildActor))))
  (Variables|Initialization|SetTileChecker _asbp_tile_checker)
  (CallFunction|SpawnGrid))

(fn ConstructionScript
  (bind _griddimension (Variables|Initialization|GetGridDimension))
  (bind (_x _y) (Utilities|Struct|BreakIntPoint _griddimension))
  (if (Variables|Default|GetbShowPreview)
    (for _index (range 0 (- _x 1))
      (for _index_2 (range 0 (- _y 1))
        (Components|InstancedStaticMesh|AddInstance (Variables|Default|GetInstancedStaticMesh) (Math|Transform|MakeTransform (Math|Vector|MakeVector (* (* _index_2 1e+02) (Variables|Initialization|GetScaleX)) (* (* _index 1e+02) (Variables|Initialization|GetScaleY)) 0.0) "0, 0, 0" (Math|Vector|MakeVector (Variables|Initialization|GetScaleX) (Variables|Initialization|GetScaleY) 1.0)))))))

(fn SpawnGrid
  (bind _returnvalue (Transformation|GetActorLocation))
  (bind _griddimension (Variables|Initialization|GetGridDimension))
  (bind (_x _y) (Utilities|Struct|BreakIntPoint _griddimension))
  (bind (_x_2 _y_2 _z) (Math|Vector|BreakVector _returnvalue))
  (for _index (range 0 (- _x 1))
    (LocalVariables|SetYInd _index)
    (for _index_2 (range 0 (- _y 1))
      (LocalVariables|SetXInd _index_2)
      (LocalVariables|SetnextLocation (Math|Vector|MakeVector (+ (* (* _index_2 1e+02) (Variables|Initialization|GetScaleX)) _x_2) (+ (* (* (LocalVariables|GetYInd) 1e+02) (Variables|Initialization|GetScaleY)) _y_2) _z))
      (LocalVariables|SettileScale (Math|Vector|MakeVector (Variables|Initialization|GetScaleX) (Variables|Initialization|GetScaleY) 1.0))
      (if (Default|CanPlaceTile (Variables|Initialization|GetTileChecker) (LocalVariables|GetnextLocation) (LocalVariables|GettileScale) "0, 0,50.000000")
        (bind _returnvalue_2 (Game|SpawnActorfromClass "/Game/Core/Grid/BP/BP_Tile.BP_Tile_C" (Math|Transform|MakeTransform (LocalVariables|GetnextLocation) (Transformation|GetActorRotation) (LocalVariables|GettileScale)) "AlwaysSpawn" 0 (Utilities|Struct|MakeIntPoint (LocalVariables|GetXInd) (LocalVariables|GetYInd)) 0))
        (Utilities|Map|Add (Variables|Initialization|GetTileMap) (Utilities|Struct|MakeIntPoint (LocalVariables|GetXInd) (LocalVariables|GetYInd)) _returnvalue_2)))))

(fn GetNeighbors
  (params (Index :type Int%20Point%20Structure) (IncludeDiagonal :type Boolean))
  (LocalVariables|Setloc_neighborIndeces (Utilities|Array|MakeArray (+ Index (Utilities|Struct|MakeIntPoint 1 0)) (+ Index (Utilities|Struct|MakeIntPoint -1 0)) (+ Index (Utilities|Struct|MakeIntPoint 0 1)) (+ Index (Utilities|Struct|MakeIntPoint 0 -1))))
  (if (not IncludeDiagonal)
    _
    (else
      (Utilities|Array|AppendArray (LocalVariables|Getloc_neighborIndeces) (Utilities|Array|MakeArray (+ Index (Utilities|Struct|MakeIntPoint 1 1)) (+ Index (Utilities|Struct|MakeIntPoint 1 -1)) (+ Index (Utilities|Struct|MakeIntPoint -1 1)) (+ Index (Utilities|Struct|MakeIntPoint -1 -1))))))
  (for _array_element (LocalVariables|Getloc_neighborIndeces)
    (if (.ReturnValue (Utilities|Map|Find (Variables|Initialization|GetTileMap) _array_element))
      (Utilities|Array|Add (LocalVariables|GetoutArr) (.Value (Utilities|Map|Find (Variables|Initialization|GetTileMap) _array_element)))))
  (return (LocalVariables|GetoutArr)))

(fn GetReachableTiles
  (params (Player :type Pawn%20Object%20Reference) (OnlyOwnTiles :type Boolean))
  ;[0 0 0] Gets all it's own tiles + neighbor tiles. Ignores blocked tiles
  (bind _values (Utilities|Map|Values (Variables|Initialization|GetTileMap)))
  (for _array_element _values
    (LocalVariables|SetLoc_CurrentTile _array_element)
    (if (and (== (Variables|/Game/Core/Grid/BP/BP_Tile.BP_Tile_C|GetOwningPlayer _array_element) Player) (Utilities|Enum|NotEqual(Enum) (Variables|/Game/Core/Grid/BP/BP_Tile.BP_Tile_C|GetState (LocalVariables|GetLoc_CurrentTile)) "NewEnumerator2"))
      (Utilities|Array|AddUnique (LocalVariables|GetoutArray) (LocalVariables|GetLoc_CurrentTile))
      (if (not OnlyOwnTiles)
        (bind _neighbors (Helper|GetNeighbors (Variables|/Game/Core/Grid/BP/BP_Tile.BP_Tile_C|GetIndex (LocalVariables|GetLoc_CurrentTile)) false))
        (for _array_element_2 _neighbors
          (LocalVariables|SetLoc_CurrentNeighbor _array_element_2)
          (if (and (!= (Variables|/Game/Core/Grid/BP/BP_Tile.BP_Tile_C|GetOwningPlayer _array_element_2) Player) (Utilities|Enum|NotEqual(Enum) (Variables|/Game/Core/Grid/BP/BP_Tile.BP_Tile_C|GetState (LocalVariables|GetLoc_CurrentNeighbor)) "NewEnumerator2"))
            (Utilities|Array|AddUnique (LocalVariables|GetoutArray) (LocalVariables|GetLoc_CurrentNeighbor)))))))
  (return (LocalVariables|GetoutArray)))

(fn PlaceUnitonTile
  (params (Unit :type Actor%20Object%20Reference) (Tile :type BP%20Tile%20Object%20Reference))
  ;[0 0 0] Make sure inputs are correct
  (bind _type (Class|BPIPlaceable|GetType(Message) Unit))
  (if (and (Utilities|Enum|Equal(Enum) _type "NewEnumerator0") (Utilities|Enum|Equal(Enum) (Variables|/Game/Core/Grid/BP/BP_Tile.BP_Tile_C|GetState Tile) "NewEnumerator0"))
    (Class|BPIPlaceable|SetTile(Message) Unit Tile)
    (Default|FillTile Tile Unit)
    (bind _returnvalue (Transformation|SetActorLocation Unit (+ (Transformation|GetActorLocation Tile) "0, 0,90.000000") false false))
    (return _returnvalue)
    (else
      (Development|PrintString "Could not place unit on tile")
      (return false))))

(fn PlaceBuildingonTile
  (params (Building :type Actor%20Object%20Reference) (Tile :type BP%20Tile%20Object%20Reference))
  ;[0 0 0] Make sure inputs are correct
  (bind _type (Class|BPIPlaceable|GetType(Message) Building))
  (if (and (Utilities|Enum|Equal(Enum) _type "NewEnumerator1") (Utilities|Enum|Equal(Enum) (Variables|/Game/Core/Grid/BP/BP_Tile.BP_Tile_C|GetState Tile) "NewEnumerator0"))
    (Default|FillTile Tile Building)
    (bind _returnvalue (Transformation|SetActorLocation Building (Transformation|GetActorLocation Tile) false false))
    (bind _asbp_base_building (Utilities|Casting|CastToBP_BaseBuilding Building))
    (Utilities|Array|Add (Variables|Default|GetBuildings) _asbp_base_building)
    (return _returnvalue)
    (else
      (Development|PrintString "Could not place building on tile")
      (return false))))