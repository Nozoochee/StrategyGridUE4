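; BP_TileChecker is a helper actor that tests whether a grid tile can be placed at a given spot.
; CanPlaceTile moves and scales the actor to the candidate location, then projects each of its Arrow components onto the navmesh with the given query extent.
; The arrows act as sample points, and the tile fails as soon as any one of them misses the navmesh.
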(fn ConstructionScript)

(fn CanPlaceTile
  (params (Location :type Vector) (Scale :type Vector) (Extent :type Vector))
  ;[0 0 0] Goes through all arrows on this actor and sees if the points are on the navmesh
  (Transformation|SetActorLocation Location false false)
  (Transformation|SetActorScale3D Scale)
  (for _array_element (Actor|GetComponentsByClass "/Script/Engine.ArrowComponent")
    (if (not (.ReturnValue (AI|Navigation|ProjectPointtoNavigation (Transformation|GetWorldLocation _array_element) 0 0 Extent)))
      (return false)))
  (return true))