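; BP_BaseBuilding is the base Blueprint for placeable buildings, tracking which player owns the building and which tile it occupies.
; SetOwningPlayer and SetTile events store those references, and matching getters return them.
; GetType returns a fixed enum value to identify the kind of placeable, and the construction script is empty.
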(event EventSetTile
  (params (NewTile :type BP%20Tile%20Object%20Reference))
  (Variables|Default|SetCurrentTile NewTile))

(event EventSetOwningPlayer
  (params (Owner :type Pawn%20Object%20Reference))
  (Variables|Default|SetOwningPlayer Owner))

(fn ConstructionScript)

(fn GetOwningPlayer
  (return (Variables|Default|GetOwningPlayer)))

(fn GetTile
  (return (Variables|Default|GetCurrentTile)))

(fn GetType
  (return "NewEnumerator1"))