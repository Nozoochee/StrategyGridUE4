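; BP_HumanPlayer is the human-controlled player in a turn-based game, providing camera-style movement and zoom.
; MoveForward and MoveRight share one world-offset path that normalizes a horizontal axis vector and scales it by MoveSpeed and frame delta time, without sweeping.
; The Zoom axis changes the spring arm length by ZoomSpeed, also scaled by delta time.
; PlayTurn is a stub that only prints a debug message.
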(event EventPlayTurn
  (Development|PrintString "HUMAN TURN"))

(event Input|AxisEvents|InputAxisMoveForward
  (params (AxisValue :type Float%20%28single-precision%29))
  (Transformation|AddActorWorldOffset (* (Math|Vector|Normalize (Math|Vector|MakeVector AxisValue (stale Input|AxisEvents|InputAxisMoveRight AxisValue) 0.0)) (* (Variables|Default|GetMoveSpeed) (Utilities|Time|GetWorldDeltaSeconds)))))

(event Input|AxisEvents|InputAxisMoveRight
  (params (AxisValue :type Float%20%28single-precision%29))
  (Transformation|AddActorWorldOffset (* (Math|Vector|Normalize (Math|Vector|MakeVector (stale Input|AxisEvents|InputAxisMoveForward AxisValue) AxisValue 0.0)) (* (Variables|Default|GetMoveSpeed) (Utilities|Time|GetWorldDeltaSeconds)))))

(event Input|AxisEvents|InputAxisZoom
  (params (AxisValue :type Float%20%28single-precision%29))
  (bind _springarm (Variables|Default|GetSpringArm))
  (Variables|/Script/Engine.SpringArmComponent|SetTargetArmLength _springarm (+ (* AxisValue (Variables|Camera|GetZoomSpeed) (Utilities|Time|GetWorldDeltaSeconds)) (Variables|/Script/Engine.SpringArmComponent|GetTargetArmLength _springarm))))

(fn ConstructionScript
  (|CallParentFunction))