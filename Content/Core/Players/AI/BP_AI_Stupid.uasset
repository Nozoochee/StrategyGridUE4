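; Simple AI player for a grid-based, turn-based game that makes every decision at random.
; Each turn, while it has fewer than three units, it async-loads a random unit class and spawns it on one of its empty tiles.
; It then moves units one at a time with delays via a recursive event, then signals turn end.
; Random tile picks retry without a limit until valid, avoiding already chosen and own occupied tiles.
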(event Custom|SpawnNewUnit
  (if (< (Utilities|Array|Length (Variables|Default|GetUnitsOnField)) 3)
    (bind _tiles (Default|GetReachableTiles (Variables|Default|GetGrid) self true))
    (Variables|Default|SetOwnTiles _tiles)
    (if (> (Utilities|Array|Length (Variables|Default|GetOwnTiles)) (Utilities|Array|Length (Variables|Default|GetUnitsOnField)))
      (bind _class (Utilities|AsyncLoadClassAsset (.Classtospawn (Utilities|Struct|BreakS_UnitData (.OutItem (Utilities|Array|Random (Variables|Default|GetAllUnits))))))
        (:Completed
          (bind _output_get (Variables|Default|SetRandomSelection (.OutItem (Utilities|Array|Random (Variables|Default|GetOwnTiles))) :!label _label))
          (if (Utilities|Enum|Equal(Enum) (Variables|/Game/Core/Grid/BP/BP_Tile.BP_Tile_C|GetState _output_get) "NewEnumerator0")
            (Default|SetActoronField (Variables|Default|GetGridGameMode) (Variables|Default|GetRandomSelection) (.AsActor (Utilities|Casting|CastToActorClass _class)))
            (CallFunction|MoveUnits)
            (else
              (goto _label)))))
      (else
        (CallFunction|MoveUnits)))
    (else
      (CallFunction|MoveUnits))))

(event Custom|MoveUnits
  ;[0.102 0 1] Start moving .5 seconds after spawning
  (Utilities|FlowControl|Delay 0.5)
  (Utilities|Set|Clear (Variables|Default|GetChosenTiles))
  (CallFunction|MoveUnit))

(event Custom|MoveUnit
  (if (not (>= (Variables|Default|Getmoved) (Utilities|Array|Length (Variables|Default|GetUnitsOnField))))
    (Variables|Default|SetUnit (Utilities|Array|Get(acopy) (Variables|Default|GetUnitsOnField) (Variables|Default|Getmoved)))
    (bind _tiles (Default|GetReachableTiles (Variables|Default|GetGrid) self false))
    (bind _output_get (Variables|Default|SetRandomSelection (.OutItem (Utilities|Array|Random _tiles)) :!label _label))
    (if (and (not (Utilities|Set|Contains (Variables|Default|GetChosenTiles) _output_get)) (or (!= (Variables|/Game/Core/Grid/BP/BP_Tile.BP_Tile_C|GetOwningPlayer (Variables|Default|GetRandomSelection)) self) (Utilities|Enum|Equal(Enum) (Variables|/Game/Core/Grid/BP/BP_Tile.BP_Tile_C|GetState (Variables|Default|GetRandomSelection)) "NewEnumerator0")))
      (Utilities|Set|Add (Variables|Default|GetChosenTiles) (Variables|Default|GetRandomSelection))
      (Default|MoveUnittoTile (Variables|Default|GetGridGameMode) (Variables|Default|GetUnit) (Variables|Default|GetRandomSelection))
      (Math|Integer|IncrementInt (Variables|Default|Getmoved)
        (:%20%20
          ;[0.102 0 1] Wait 1 sec to make turn easier to follow
          (Utilities|FlowControl|Delay 1.0)
          (CallFunction|MoveUnit)))
      (else
        (goto _label)))
    (else
      ;[1 0.05503 0] Don't forget this!
      (Default|CallOnTurnEnd))))

(event EventBeginPlay
  (|CallParentFunction))

(event EventPlayTurn
  ;[0 0 0] AI logic goes here. Make sure to call OnTurnEnd when it's done.
  (|CallParentFunction)
  (Variables|Default|Setmoved 0)
  (CallFunction|SpawnNewUnit))

(fn ConstructionScript
  (|CallParentFunction))