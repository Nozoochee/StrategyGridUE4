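; Base Blueprint for an AI player in a grid-based, turn-based game with units and buildings.
; On BeginPlay it stores a reference to the BP_GridManager actor and loads every row of DT_Units and DT_Buildings into its AllUnits and AllBuildings arrays.
; PlayTurn is a placeholder that only prints a debug message and does not yet use the cached data.
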(event EventPlayTurn
  (Development|PrintString "AI TURN"))

(event EventBeginPlay
  (|CallParentFunction)
  (bind _returnvalue (Actor|GetActorOfClass "/Game/Core/Grid/BP/BP_GridManager.BP_GridManager_C"))
  (Variables|Default|SetGrid _returnvalue)
  ;[0 0 0] Gets all buildings and units that are in the game
  (bind _outrownames (DataTable|GetDataTableRowNames "/Game/Core/Placeables/Units/DT_Units.DT_Units"))
  (for _array_element _outrownames
    (bind _returnvalue_2 (Utilities|GetDataTableRow "/Game/Core/Placeables/Units/DT_Units.DT_Units" _array_element)
      (:then
        (Utilities|Array|Add (Variables|Default|GetAllUnits) _returnvalue_2))))
  (bind _outrownames_2 (DataTable|GetDataTableRowNames "/Game/Core/Placeables/Buildings/DT_Buildings.DT_Buildings"))
  (for _array_element_2 _outrownames_2
    (bind _returnvalue_3 (Utilities|GetDataTableRow "/Game/Core/Placeables/Buildings/DT_Buildings.DT_Buildings" _array_element_2)
      (:then
        (Utilities|Array|Add (Variables|Default|GetAllBuildings) _returnvalue_3)))))

(fn ConstructionScript
  (|CallParentFunction))